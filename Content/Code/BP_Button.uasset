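; BP_Button is an interactable button that pauses and resumes a Rotator, with visual and audio feedback.
; Capsule overlap sets the Active flag and shows or hides the PSHint prompt.
; Each Interact call alternates through a FlipFlop, pausing first, then unpausing, swapping the sphere between inactive and active materials.
; Each toggle plays its own blip sound, with volume adjusted through the Game Instance.
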(event OnComponentBeginOverlap(Capsule)
  (params (OverlappedComponent :type Primitive%20Component%20Object%20Reference) (OtherActor :type Actor%20Object%20Reference) (OtherComp :type Primitive%20Component%20Object%20Reference) (OtherBodyIndex :type Integer) (bFromSweep :type Boolean) (SweepResult :type Hit%20Result%20Structure%20%28by%20ref%29))
  (Variables|Default|SetActive true)
  (Rendering|SetVisibility (Variables|Default|GetPS_Hint) true false))

(event OnComponentEndOverlap(Capsule)
  (params (OverlappedComponent :type Primitive%20Component%20Object%20Reference) (OtherActor :type Actor%20Object%20Reference) (OtherComp :type Primitive%20Component%20Object%20Reference) (OtherBodyIndex :type Integer))
  (Variables|Default|SetActive false)
  (Rendering|SetVisibility (Variables|Default|GetPS_Hint) false false))

(event EventInteract
  (bind _returnvalue (Game|GetGameInstance))
  (bind _sphere (Variables|Default|GetSphere))
  (bind _rotator (Variables|Default|GetRotator))
  (Utilities|FlowControl|FlipFlop
    (:A
      (Default|Pause _rotator)
      (Rendering|Material|SetMaterial _sphere 0 "/Game/Data/Materials/MI_Inactive.MI_Inactive")
      (bind _volumemultiplier (Utilities|AdjustSoundVolume _returnvalue))
      (Audio|PlaySound2D "/Game/Data/SoundEffects/S_BlipSelect01.S_BlipSelect01" _volumemultiplier 1.0 0.0 0 0 false))
    (:B
      (Default|Unpause _rotator)
      (Rendering|Material|SetMaterial _sphere 0 "/Game/Data/Materials/MI_Active.MI_Active")
      (bind _volumemultiplier_2 (Utilities|AdjustSoundVolume _returnvalue))
      (Audio|PlaySound2D "/Game/Data/SoundEffects/S_BlipSelect02.S_BlipSelect02" _volumemultiplier_2 1.0 0.0 0 0 false))))

(fn ConstructionScript)