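; BP_PickUp is a collectible that adds to a star count when the player touches it.
; On cube overlap while active, it checks for BP_Player and increments the GameInstance's StarCount map entry keyed by the EndPoint's current main version.
; It then plays a coin sound, hides itself and deactivates rather than being destroyed, so the Activate event can show and re-arm it.
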(event OnComponentBeginOverlap(Cube)
  (params (OverlappedComponent :type Primitive%20Component%20Object%20Reference) (OtherActor :type Actor%20Object%20Reference) (OtherComp :type Primitive%20Component%20Object%20Reference) (OtherBodyIndex :type Integer) (bFromSweep :type Boolean) (SweepResult :type Hit%20Result%20Structure%20%28by%20ref%29))
  (bind _endpoint (Variables|Default|GetEndPoint))
  (bind _currentmainversion (Variables|/Game/Code/Saving/BP_EndPoint.BP_EndPoint_C|GetCurrentMainVersion _endpoint))
  (if (Variables|Default|GetActive)
    (Utilities|Casting|CastToBP_Player OtherActor)
    (bind _asbp_game_instance (Utilities|Casting|CastToBP_GameInstance (Game|GetGameInstance)))
    (bind _result (Math|Integer|IncrementInt (.Value (Utilities|Map|Find (Utilities|Struct|BreakSGameDetails (Variables|/Game/Base/BP_GameInstance.BP_GameInstance_C|GetGameDetails _asbp_game_instance)) _currentmainversion)))
      (:%20%20
        (Utilities|Map|Add (Utilities|Struct|BreakSGameDetails (Variables|/Game/Base/BP_GameInstance.BP_GameInstance_C|GetGameDetails _asbp_game_instance)) _currentmainversion _result)
        (Audio|PlaySound2D "/Game/Data/Sound/SoundEffects/S_PickupCoin02.S_PickupCoin02" 1.0 1.0 0.0 0 0 false)
        (Rendering|SetActorHiddenInGame true)
        (Variables|Default|SetActive false)))))

(event Custom|Activate
  (Variables|Default|SetActive true)
  (Rendering|SetActorHiddenInGame false))

(fn ConstructionScript
  (|CallParentFunction))