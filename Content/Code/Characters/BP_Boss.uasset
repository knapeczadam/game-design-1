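; Boss character whose two eye components periodically spin and which is flagged as dead when hit by a projectile.
; A looping timer captures both eyes' world rotations, then a timeline lerps their roll a quarter turn in opposite directions.
; A capsule hit from a BP_Projectile only clears IsAlive; this graph does not act on that flag.
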(event OnComponentHit(CapsuleComponent)
  (params (HitComponent :type Primitive%20Component%20Object%20Reference) (OtherActor :type Actor%20Object%20Reference) (OtherComp :type Primitive%20Component%20Object%20Reference) (NormalImpulse :type Vector :default "0, 0, 0") (Hit :type Hit%20Result%20Structure%20%28by%20ref%29))
  (Utilities|Casting|CastToBP_Projectile OtherActor)
  (Variables|Default|SetIsAlive false))

(event Custom|RotateEyes
  (bind _output_get (Variables|Default|SetStartRotation1 (Transformation|GetWorldRotation (Variables|Default|GetEyes))))
  (bind _output_get_2 (Variables|Default|SetStartRotation2 (Transformation|GetWorldRotation (Variables|Default|GetEyes1))))
  (Variables|Default|SetEndRotation1 (Math|Rotator|MakeRotator (+ (.roll _output_get) (Math|Float|MakeLiteralFloat 9e+01)) (.pitch _output_get) (.yaw _output_get)))
  (Variables|Default|SetEndRotation2 (Math|Rotator|MakeRotator (+ (.roll _output_get_2) (Math|Float|MakeLiteralFloat -9e+01)) (.pitch _output_get_2) (.yaw _output_get_2)))
  (bind _0_1 (Timeline|RotatorTimeline PlayFromStart)
    (:Update
      (Transformation|SetWorldRotation (Variables|Default|GetEyes) (Math|Rotator|Lerp(Rotator) (Variables|Default|GetStartRotation1) (Variables|Default|GetEndRotation1) (Math|Float|MapRangeClamped _0_1 0.0 (Components|Timeline|GetTimelineLength (Variables|Default|GetRotatorTimeline)) 0.0 1.0)) false false)
      (Transformation|SetWorldRotation (Variables|Default|GetEyes1) (Math|Rotator|Lerp(Rotator) (Variables|Default|GetStartRotation2) (Variables|Default|GetEndRotation2) (Math|Float|MapRangeClamped _0_1 0.0 (Components|Timeline|GetTimelineLength (Variables|Default|GetRotatorTimeline)) 0.0 1.0)) false false))))

(event EventBeginPlay
  (|CallParentFunction)
  (Utilities|Time|SetTimerbyEvent (delegate Custom|RotateEyes) 5.0 true))

(event Collision|EventActorBeginOverlap
  (params (OtherActor :type Actor%20Object%20Reference))
  (|CallParentFunction OtherActor))

(event EventTick
  (params (DeltaSeconds :type Float%20%28single-precision%29))
  (|CallParentFunction DeltaSeconds))

(fn ConstructionScript
  (|CallParentFunction))