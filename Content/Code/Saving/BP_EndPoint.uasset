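; Level exit actor that saves the game and loads the configured next level when an overlapping BP_BaseCharacter enters it while active.
; Activate, callable directly or optionally fired by TriggerBox overlap, runs once to set the active flag, swap the plane material and magic particles, and play a volume-adjusted sound.
; The exit overlap also runs once, saving at the actor's transform through BP_TopDownGameMode, then opening the level after a short delay.
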(event OnComponentBeginOverlap(TriggerBox)
  (params (OverlappedComponent :type Primitive%20Component%20Object%20Reference) (OtherActor :type Actor%20Object%20Reference) (OtherComp :type Primitive%20Component%20Object%20Reference) (OtherBodyIndex :type Integer) (bFromSweep :type Boolean) (SweepResult :type Hit%20Result%20Structure%20%28by%20ref%29))
  (if (Variables|Default|GetActivateByTriggerBox)
    (Utilities|Casting|CastToBP_BaseCharacter OtherActor)
    (CallFunction|Activate)))

(event Custom|Activate
  (Utilities|FlowControl|DoOnce false
    (:Completed
      (Rendering|Material|SetMaterial (Variables|Default|GetPlane) 0 "/Game/Data/Materials/MI_Active.MI_Active")
      (Variables|Default|SetIsActive true)
      (Rendering|SetVisibility (Variables|Default|GetPS_Magic_Active) true false)
      (Rendering|SetVisibility (Variables|Default|GetPS_Magic_Inactive) false false)
      (bind _volumemultiplier (Utilities|AdjustSoundVolume (Game|GetGameInstance)))
      (Audio|PlaySound2D "/Game/Data/SoundEffects/S_PickupCoin02.S_PickupCoin02" _volumemultiplier 0.2 0.0 0 0 false))))

(event Collision|EventActorBeginOverlap
  (params (OtherActor :type Actor%20Object%20Reference))
  (if (Variables|Default|GetIsActive)
    (Utilities|Casting|CastToBP_BaseCharacter OtherActor)
    (Utilities|FlowControl|DoOnce false
      (:Completed
        (Utilities|Casting|CastToBP_TopDownGameMode (Game|GetGameMode))
        (CallFunction|SaveGameatLocation (Transformation|GetActorTransform))
        (Utilities|FlowControl|Delay 1.5)
        (Game|OpenLevel(byName) (Variables|Default|GetLevelToLoad))))))

(event EventTick
  (params (DeltaSeconds :type Float%20%28single-precision%29)))

(fn ConstructionScript)