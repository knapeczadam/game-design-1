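; BP_TrapButton is a one-shot interactable button, named for traps, that shows whether it is still active.
; Interact passes a DoOnce gate, clears Active, triggers a single Rotator turn, swaps the Sphere to the inactive material and plays a blip sound.
; NewReset restores Active and the active material and reopens the gate, while BeginPlay stops the Rotator.
; The graph itself references no trap.
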(event Custom|NewReset
  (Variables|Default|SetActive true)
  (Rendering|Material|SetMaterial (Variables|Default|GetSphere) 0 "/Game/Data/Materials/MI_Active.MI_Active")
  (Utilities|FlowControl|DoOnce false) ; enters at Reset
)

(event EventBeginPlay
  (Default|Stop (Variables|Default|GetRotator)))

(event EventInteract
  (Utilities|FlowControl|DoOnce false
    (:Completed
      (Variables|Default|SetActive false)
      (Default|RotateOnce (Variables|Default|GetRotator))
      (Rendering|Material|SetMaterial (Variables|Default|GetSphere) 0 "/Game/Data/Materials/MI_Inactive.MI_Inactive")
      (Audio|PlaySound2D "/Game/Data/Sound/SoundEffects/S_BlipSelect01.S_BlipSelect01" 1.0 1.0 0.0 0 0 false))))

(fn ConstructionScript
  (|CallParentFunction))