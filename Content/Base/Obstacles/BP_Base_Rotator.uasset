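; Base rotating obstacle that turns its Sphere component by a set rotation on a looping timer, optionally starting immediately on BeginPlay.
; Each step lerps from the current actor rotation via a timeline, either always adding the rotation or flip-flopping between adding and subtracting it.
; The Long option swaps in a longer linear curve and timeline length at BeginPlay.
; Stop, Pause and Unpause events control the timer.
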(event Custom|Stop
  (Utilities|Time|ClearandInvalidateTimerbyHandle (stale EventBeginPlay _returnvalue)))

(event Custom|Rotate
  (bind _rotation (Variables|Default|GetRotation))
  (bind _rotation_2 (Variables|Default|GetRotation))
  (bind _rotation_3 (Variables|Default|GetRotation))
  (bind _output_get (Variables|Default|SetStart%20Rotation (Transformation|GetActorRotation)))
  (if (Variables|Default|GetFullRotation)
    (Variables|Default|SetEnd%20Rotation (Math|Rotator|MakeRotator (+ (.roll _output_get) (.roll _rotation_3)) (+ (.pitch _output_get) (.pitch _rotation_3)) (+ (.yaw _output_get) (.yaw _rotation_3))))
    (bind _0_1 (Timeline|RotatorTimeline PlayFromStart)
      (:Update
        (Transformation|SetWorldRotation (Variables|Default|GetSphere) (Math|Rotator|Lerp(Rotator) (Variables|Default|GetStart%20Rotation) (Variables|Default|GetEnd%20Rotation) (Math|Float|MapRangeClamped _0_1 0.0 (Components|Timeline|GetTimelineLength (Variables|Default|GetRotatorTimeline)) 0.0 1.0)) false false)))
    (else
      (Utilities|FlowControl|FlipFlop
        (:A
          (Variables|Default|SetEnd%20Rotation (Math|Rotator|MakeRotator (+ (.roll _output_get) (.roll _rotation_2)) (+ (.pitch _output_get) (.pitch _rotation_2)) (+ (.yaw _output_get) (.yaw _rotation_2))))
          (Timeline|RotatorTimeline PlayFromStart))
        (:B
          (Variables|Default|SetEnd%20Rotation (Math|Rotator|MakeRotator (- (.roll _output_get) (.roll _rotation)) (- (.pitch _output_get) (.pitch _rotation)) (- (.yaw _output_get) (.yaw _rotation))))
          (Timeline|RotatorTimeline PlayFromStart))))))

(event Custom|Pause
  (Utilities|Time|PauseTimerbyHandle (stale EventBeginPlay _returnvalue)))

(event Custom|Unpause
  (Utilities|Time|UnpauseTimerbyHandle (stale EventBeginPlay _returnvalue)))

(event EventBeginPlay
  (bind _rotatortimeline (Variables|Default|GetRotatorTimeline))
  (Utilities|FlowControl|Sequence
    (:then_0
      (if (Variables|Default|GetLong)
        (Components|Timeline|SetTimelineLength _rotatortimeline 2.0)
        (Class|TimelineComponent|SetFloatCurve _rotatortimeline "/Game/Base/Obstacles/LinearLong.LinearLong" "0-1")))
    (:then_1
      (bind _returnvalue (Utilities|Time|SetTimerbyEvent (delegate Custom|Rotate) (Variables|Default|GetInterval) true))
      (if (Variables|Default|GetStartFromBeginPlay)
        (CallFunction|Rotate)))))

(event Collision|EventActorBeginOverlap
  (params (OtherActor :type Actor%20Object%20Reference))
  ;[1 1 1] Comment
)

(event EventTick
  (params (DeltaSeconds :type Float%20%28single-precision%29)))

(fn ConstructionScript)