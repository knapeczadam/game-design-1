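; BP_Rotator is an obstacle actor with a Cube component that makes a yaw turn on a repeating timer.
; A looping timer started on BeginPlay fires Rotate every few seconds, capturing the actor's rotation and a target a quarter turn further in yaw.
; A timeline then lerps the Cube's world rotation between the two.
; Cube overlaps only print a debug string.
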(event OnComponentBeginOverlap(Cube)
  (params (OverlappedComponent :type Primitive%20Component%20Object%20Reference) (OtherActor :type Actor%20Object%20Reference) (OtherComp :type Primitive%20Component%20Object%20Reference) (OtherBodyIndex :type Integer) (bFromSweep :type Boolean) (SweepResult :type Hit%20Result%20Structure%20%28by%20ref%29))
  (Development|PrintString "Hello"))

(event Custom|Rotate
  (bind _output_get (Variables|Default|SetStart%20Rotation (Transformation|GetActorRotation)))
  (Variables|Default|SetEnd%20Rotation (Math|Rotator|MakeRotator 0.0 0.0 (+ (.yaw _output_get) 9e+01)))
  (bind _0_1 (Timeline|Timeline PlayFromStart)
    (:Update
      (Transformation|SetWorldRotation (Variables|Default|GetCube) (Math|Rotator|Lerp(Rotator) (Variables|Default|GetStart%20Rotation) (Variables|Default|GetEnd%20Rotation) _0_1) false false))))

(event EventBeginPlay
  (Utilities|Time|SetTimerbyEvent (delegate Custom|Rotate) 5.0 true))

(event Collision|EventActorBeginOverlap
  (params (OtherActor :type Actor%20Object%20Reference)))

(event EventTick
  (params (DeltaSeconds :type Float%20%28single-precision%29)))

(fn ConstructionScript)